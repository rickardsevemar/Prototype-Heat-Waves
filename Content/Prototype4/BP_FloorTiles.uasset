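; Floor tile actor for the Heat Waves prototype that extends the track as the player pawn moves across it.
; When Pawn_Heatwaves overlaps its box, it asks GM_HeatWaves to add another tile, then destroys itself after a short delay.
; GetArrowTransform exposes the Arrow's world transform.
; Tick polls PC_HeatWaves Day and Night flags to show HW components by day and spotlights by night.
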(event OnComponentBeginOverlap(Box)
  (params (OverlappedComponent :type Primitive%20Component%20Object%20Reference) (OtherActor :type Actor%20Object%20Reference) (OtherComp :type Primitive%20Component%20Object%20Reference) (OtherBodyIndex :type Integer) (bFromSweep :type Boolean) (SweepResult :type Hit%20Result%20Structure%20%28by%20ref%29))
  (Utilities|Casting|CastToPawn_Heatwaves OtherActor)
  (bind _asgm_heat_waves (Utilities|Casting|CastToGM_HeatWaves (Game|GetGameMode)))
  (Default|AddFloorTile _asgm_heat_waves)
  (Utilities|FlowControl|Delay 2.0)
  (Actor|DestroyActor))

(event EventBeginPlay
  (bind _aspc_heat_waves (Utilities|Casting|CastToPC_HeatWaves (Game|GetPlayerController 0)))
  (Variables|Default|SetAs%20PC%20Heat%20Waves _aspc_heat_waves))

(event EventTick
  (params (DeltaSeconds :type Float%20%28single-precision%29))
  (if (Variables|/Game/Prototype4/PC_HeatWaves.PC_HeatWaves_C|GetDay (Variables|Default|GetAs%20PC%20Heat%20Waves))
    (Rendering|SetVisibility (Variables|Default|GetHW1) true false)
    (Rendering|SetVisibility (Variables|Default|GetHW2) true false)
    (Rendering|SetVisibility (Variables|Default|GetHW3) true false)
    (Rendering|SetVisibility (Variables|Default|GetHW4) true false)
    (Rendering|SetVisibility (Variables|Default|GetSpotLight1) false false)
    (Rendering|SetVisibility (Variables|Default|GetSpotLight) false false)
    (elif (Variables|/Game/Prototype4/PC_HeatWaves.PC_HeatWaves_C|GetNight (Variables|Default|GetAs%20PC%20Heat%20Waves))
      (Rendering|SetVisibility (Variables|Default|GetHW1) false false)
      (Rendering|SetVisibility (Variables|Default|GetHW2) false false)
      (Rendering|SetVisibility (Variables|Default|GetHW3) false false)
      (Rendering|SetVisibility (Variables|Default|GetHW4) false false)
      (Rendering|SetVisibility (Variables|Default|GetSpotLight1) true false)
      (Rendering|SetVisibility (Variables|Default|GetSpotLight) true false))))

(fn ConstructionScript)

(fn GetArrowTransform
  (return (Transformation|GetWorldTransform (Variables|Default|GetArrow))))