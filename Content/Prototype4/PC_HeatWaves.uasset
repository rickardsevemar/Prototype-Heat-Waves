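; Player controller for the HeatWaves prototype that adds the HUD widget, controls the speed of time and tracks day or night.
; On BeginPlay it caches the custom sun sky actor and game state.
; The mouse wheel steps the game state's seconds added per tick up or down within limits, including negative values.
; Every tick it reads the sky's hour to set Day and Night flags, treating 8 to 18 as day.
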(event Custom|CheckDayAndNight
  (if (>= (Variables|/Game/Prototype4/Assets/BP_CustomSunSky.BP_CustomSunSky_C|GetHours (Variables|Default|GetSunSky)) 8)
    (if (<= (Variables|/Game/Prototype4/Assets/BP_CustomSunSky.BP_CustomSunSky_C|GetHours (Variables|Default|GetSunSky)) 18)
      (Variables|Default|SetDay true)
      (Variables|Default|SetNight false)
      (else
        (Variables|Default|SetNight true :!label _label)
        (Variables|Default|SetDay false)))
    (else
      (goto _label))))

(event EventBeginPlay
  (bind _returnvalue (UserInterface|CreateWidget "/Game/Prototype4/W_HeatWaves.W_HeatWaves_C"))
  (UserInterface|Viewport|AddtoViewport _returnvalue 0)
  (bind _returnvalue_2 (Actor|GetActorOfClass "/Game/Prototype4/Assets/BP_CustomSunSky.BP_CustomSunSky_C"))
  (Variables|Default|SetSunSky _returnvalue_2)
  (bind _asbp_custom_game_state (Utilities|Casting|CastToBP_CustomGameSTate (Game|GetGameState)))
  (Variables|Default|SetAs%20BP%20Custom%20Game%20STate _asbp_custom_game_state))

(event EventTick
  (params (DeltaSeconds :type Float%20%28single-precision%29))
  (CallFunction|CheckDayandNight))

(event Input|MouseEvents|MouseWheelUp
  (params (Key :type Key%20Structure :default "None"))
  (bind _as_bp_custom_game_state (Variables|Default|GetAs%20BP%20Custom%20Game%20STate))
  (:Pressed
    (if (< (Variables|/Game/Prototype4/Assets/BP_CustomGameSTate.BP_CustomGameSTate_C|GetAmountOfSecondsToAddPerTick (Variables|Default|GetAs%20BP%20Custom%20Game%20STate)) 180)
      (Variables|/Game/Prototype4/Assets/BP_CustomGameSTate.BP_CustomGameSTate_C|SetAmountOfSecondsToAddPerTick _as_bp_custom_game_state (+ (Variables|/Game/Prototype4/Assets/BP_CustomGameSTate.BP_CustomGameSTate_C|GetAmountOfSecondsToAddPerTick _as_bp_custom_game_state) 20)))))

(event Input|MouseEvents|MouseWheelDown
  (params (Key :type Key%20Structure :default "None"))
  (bind _as_bp_custom_game_state (Variables|Default|GetAs%20BP%20Custom%20Game%20STate))
  (:Pressed
    (if (> (Variables|/Game/Prototype4/Assets/BP_CustomGameSTate.BP_CustomGameSTate_C|GetAmountOfSecondsToAddPerTick (Variables|Default|GetAs%20BP%20Custom%20Game%20STate)) -180)
      (Variables|/Game/Prototype4/Assets/BP_CustomGameSTate.BP_CustomGameSTate_C|SetAmountOfSecondsToAddPerTick _as_bp_custom_game_state (- (Variables|/Game/Prototype4/Assets/BP_CustomGameSTate.BP_CustomGameSTate_C|GetAmountOfSecondsToAddPerTick _as_bp_custom_game_state) 20)))))

(fn ConstructionScript)