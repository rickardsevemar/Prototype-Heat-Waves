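; GM_HeatWaves is the Prototype4 game mode, which lays out the starting stretch of floor and environment tiles when play begins.
; BeginPlay runs a short loop that calls AddFloorTile and AddEnvironmentTile to spawn BP_FloorTiles and BP_Environment actors.
; Each spawn stores the new tile's arrow transform as the next spawn point, so the floor and environment form two independently chained sequences.
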(event EventBeginPlay
  (for _index (range 0 3)
    (CallFunction|AddFloorTile)
    (CallFunction|AddEnvironmentTile)))

(event EventTick
  (params (DeltaSeconds :type Float%20%28single-precision%29)))

(fn ConstructionScript)

(fn AddFloorTile
  (bind _returnvalue (Game|SpawnActorfromClass "/Game/Prototype4/BP_FloorTiles.BP_FloorTiles_C" (Variables|Default|GetNextRoadSpawnPoint) "Undefined" 0 0))
  (bind _arrowtrans (Default|GetArrowTransform _returnvalue))
  (Variables|Default|SetNextRoadSpawnPoint _arrowtrans))

(fn AddEnvironmentTile
  (bind _returnvalue (Game|SpawnActorfromClass "/Game/Prototype4/BP_Environment.BP_Environment_C" (Variables|Default|GetNextEnvironmentSpawnPoint) "Undefined" 0 0))
  (bind _spawntrans (Default|GetArrowTransform _returnvalue))
  (Variables|Default|SetNextEnvironmentSpawnPoint _spawntrans))