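; BP_CustomGameSTate is a game state Blueprint that runs the time-of-day clock for the level's BP_CustomSunSky.
; On BeginPlay it converts the sky actor's current time to total seconds and starts a looping timer at a configurable tick rate.
; Each tick adds a set increment and writes hours, minutes and seconds back through timespans.
; The day reset compares that increment, not the accumulated time, against one day.
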(event Custom|TimeUpdate
  (bind _sun_sky (Variables|Default|GetSun%20Sky))
  (bind _output_get (Variables|Default|SetTimeOfDayInSeconds (+ (Variables|Default|GetTimeOfDayInSeconds) (Variables|Default|GetAmountOfSecondsToAddPerTick))))
  (Variables|/Game/Prototype4/Assets/BP_CustomSunSky.BP_CustomSunSky_C|SetHours _sun_sky (.Hours (Math|Timespan|BreakTimespan (Math|Timespan|MakeTimespan 0 0 0 _output_get))))
  (Variables|/Game/Prototype4/Assets/BP_CustomSunSky.BP_CustomSunSky_C|SetMinutes _sun_sky (.Minutes (Math|Timespan|BreakTimespan (Math|Timespan|MakeTimespan 0 0 0 _output_get))))
  (Variables|/Game/Prototype4/Assets/BP_CustomSunSky.BP_CustomSunSky_C|SetSeconds _sun_sky (.Seconds (Math|Timespan|BreakTimespan (Math|Timespan|MakeTimespan 0 0 0 _output_get))))
  (if (>= (Variables|Default|GetAmountOfSecondsToAddPerTick) 86400)
    (Variables|Default|SetTimeOfDayInSeconds 0)))

(event EventBeginPlay
  (bind _returnvalue (Actor|GetActorOfClass "/Game/Prototype4/Assets/BP_CustomSunSky.BP_CustomSunSky_C"))
  (bind _output_get (Variables|Default|SetSun%20Sky _returnvalue))
  (Variables|Default|SetTimeOfDayInSeconds (Math|Float|Truncate (Math|Timespan|GetTotalSeconds (Math|Timespan|MakeTimespan 0 (Variables|/Game/Prototype4/Assets/BP_CustomSunSky.BP_CustomSunSky_C|GetHours _output_get) (Variables|/Game/Prototype4/Assets/BP_CustomSunSky.BP_CustomSunSky_C|GetMinutes _output_get) (Variables|/Game/Prototype4/Assets/BP_CustomSunSky.BP_CustomSunSky_C|GetSeconds _output_get)))))
  (Utilities|Time|SetTimerbyEvent (delegate Custom|TimeUpdate) (/ 1.0 (Variables|Default|GetAmountToTickASecond)) true))

(fn ConstructionScript)