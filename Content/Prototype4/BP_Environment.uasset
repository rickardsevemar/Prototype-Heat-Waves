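; BP_Environment is an environment tile actor for the HeatWaves prototype, forming part of a continuously spawned track.
; When the Heatwaves pawn overlaps its Box trigger, it asks the GM_HeatWaves game mode to add another tile, then destroys itself after a five-second delay.
; GetArrowTransform exposes the world transform of its Arrow component.
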(event OnComponentBeginOverlap(Box)
  (params (OverlappedComponent :type Primitive%20Component%20Object%20Reference) (OtherActor :type Actor%20Object%20Reference) (OtherComp :type Primitive%20Component%20Object%20Reference) (OtherBodyIndex :type Integer) (bFromSweep :type Boolean) (SweepResult :type Hit%20Result%20Structure%20%28by%20ref%29))
  (Utilities|Casting|CastToPawn_Heatwaves OtherActor)
  (Default|AddEnvironmentTile (Variables|Default|GetAs%20GM%20Heat%20Waves))
  (Utilities|FlowControl|Delay 5.0)
  (Actor|DestroyActor))

(event EventBeginPlay
  (bind _asgm_heat_waves (Utilities|Casting|CastToGM_HeatWaves (Game|GetGameMode)))
  (Variables|Default|SetAs%20GM%20Heat%20Waves _asgm_heat_waves))

(event Collision|EventActorBeginOverlap
  (params (OtherActor :type Actor%20Object%20Reference)))

(event EventTick
  (params (DeltaSeconds :type Float%20%28single-precision%29)))

(fn ConstructionScript)

(fn GetArrowTransform
  (return (Transformation|GetWorldTransform (Variables|Default|GetArrow))))